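; BP_BaseEnemyBlur is an enemy that damages the player with melee attacks and reports its death to the hordes manager.
; While attacking, Tick checks the attack collision against the player pawn, using a DoOnce to apply damage once per overlap to the player's HealthComponent.
; Its own HealthComponent triggers death, which notifies BP_HordesManager and the AI controller, plays a sound, spins the actor via timeline and destroys it after a delay.
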(event Custom|Dead
  (bind _returnvalue (Actor|GetActorOfClass "/Game/HordesManager/BP_HordesManager.BP_HordesManager_C"))
  (Default|CallOnEnemyDie _returnvalue)
  (bind _asbp_enemy_controller (Utilities|Casting|CastToBP_EnemyController (Pawn|GetController)))
  (Default|Dead _asbp_enemy_controller)
  (Variables|Default|SetIsDead true)
  (Audio|PlaySound2D "/Game/JoaquinGraciosin/Musica/Risa1.Risa1" 1.0 1.0 0.0 0 0)
  (bind _spin (Timeline|Spin Play)
    (:Update
      (Transformation|SetActorRotation (Math|Rotator|MakeRotator 0.0 0.0 _spin))
      (Utilities|FlowControl|Delay 2.0)
      (Actor|DestroyActor))))

(event EventBeginPlay
  (EventDispatchers|BindEventtoFDead (Variables|Default|GetHealthComponent) (delegate Custom|Dead)))

(event Collision|EventActorBeginOverlap
  (params (OtherActor :type Actor%20Object%20Reference)))

(event EventTick
  (params (DeltaSeconds :type Float%20%28single-precision%29))
  (if (and (Collision|IsOverlappingActor (Variables|Default|GetCollisionAttack) (Game|Player|GetPlayerPawn 0) :!class /Script/Engine.PrimitiveComponent) (Variables|Default|GetIsAttacking))
    (Utilities|FlowControl|DoOnce false :!label _label
      (:Completed
        (bind _asbp_my_player_character (Utilities|Casting|CastToBP_MyPlayerCharacter (Game|Player|GetPlayerPawn 0)))
        (Default|DamageEvent (Variables|/Game/JoaquinGraciosin/Blueprints/Player/BP_MyPlayerCharacter.BP_MyPlayerCharacter_C|GetHealthComponent _asbp_my_player_character) (Variables|Default|GetDamage))))
    (else
      (goto _label Reset))))

(fn ConstructionScript)